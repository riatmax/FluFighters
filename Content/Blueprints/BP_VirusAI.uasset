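; BP_VirusAI is an enemy that chases the player and damages them on contact.
; When pawn sensing spots a pawn, it sets a seen flag and issues an AI move to the player character, with no logic here to clear the flag.
; Capsule hits on the first-person character call its LoseHealth and set an attacking flag.
; LoseEnemyHealth subtracts damage and, at zero, prints a debug string and destroys the actor after a short delay.
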(event OnSeePawn(PawnSensing)
  (params (Pawn :type Pawn%20Object%20Reference))
  (Variables|Default|SetIsSeeingPlayer true)
  (CallFunction|FollowPlayer))

(event OnComponentHit(CapsuleComponent)
  (params (HitComponent :type Primitive%20Component%20Object%20Reference) (OtherActor :type Actor%20Object%20Reference) (OtherComp :type Primitive%20Component%20Object%20Reference) (NormalImpulse :type Vector :default "0, 0, 0") (Hit :type Hit%20Result%20Structure%20%28by%20ref%29))
  (bind _asbp_first_person_character (Utilities|Casting|CastToBP_FirstPersonCharacter OtherActor))
  (Default|LoseHealth _asbp_first_person_character (Variables|Default|GetEnemyDamage))
  (Variables|Default|SetIsAttacking true))

(event Custom|FollowPlayer
  (if (Variables|Default|GetIsSeeingPlayer)
    (AI|AIMoveTo self "0, 0, 0" (Game|GetPlayerCharacter 0) 5.0 false)))

(event Custom|LoseEnemyHealth
  (params (Damage :type Integer))
  (bind _output_get (Variables|Default|SetEnemyHealth (- (Variables|Default|GetEnemyHealth) Damage)))
  (if (<= _output_get 0.0)
    (Development|PrintString "Hello")
    (Utilities|FlowControl|Delay 2.0)
    (Actor|DestroyActor)))

(fn ConstructionScript)